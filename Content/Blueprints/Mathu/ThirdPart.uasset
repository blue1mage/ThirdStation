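; Actor that displays one entry from a text list in a matching color and lets overlapping actors cycle through the list.
; Its text starts blank, and SetView applies the current index's string and color to the TextRender.
; While Show is true, overlapping the bottom Box steps forward and the top Box1 steps back, wrapping at both ends.
; setShow clears Show, which stops cycling, and displays the current entry.
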(event `setShow`
  (set `self.Show` false)
  (`self.Set View`))

(event `self.ReceiveBeginPlay`
  (`TextRenderComponent.K2_SetText` (`self.TextRender`) (`KismetTextLibrary.Conv_StringToText` "")))

(event `Set View`
  (bind _index (`self.index`))
  (bind _textrender (`self.TextRender`))
  (`TextRenderComponent.K2_SetText` _textrender (`|GetArrayItem` (`self.ListArr`) _index))
  (`TextRenderComponent.SetTextRenderColor` _textrender (`|GetArrayItem` (`self.Color array`) _index)))

(event `self.ReceiveActorBeginOverlap`
  (params (OtherActor :type "Actor Object Reference"))
  (bind _returnvalue (- (`self.Index`) 1))
  (if (`self.Show`)
    ;[1 1 1] on the bottom box overlap
    (if (`PrimitiveComponent.IsOverlappingActor` (`self.Box`) OtherActor)
      (set `self.Index` (mod (+ (`self.Index`) 1) (`KismetArrayLibrary.Array_Length` (`self.ListArr`))))
      (`self.Set View`)
      (else
        ;[1 1 1] top box overlap
        (if (`PrimitiveComponent.IsOverlappingActor` (`self.Box1`) OtherActor)
          (if (< _returnvalue 0)
            (bind _result (`/Engine/EditorBlueprintResources/StandardMacros.DecrementInt` (`KismetArrayLibrary.Array_Length` (`self.ListArr`)))
              (:`  `
                (set `self.Index` _result)))
            (else
              (set `self.Index` _returnvalue)))
          (`self.Set View`))))))

(fn `UserConstructionScript`)