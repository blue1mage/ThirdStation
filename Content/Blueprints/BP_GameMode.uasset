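; Game mode that tracks completion progress and reveals the "MatThu" pieces and their hint once three completions are recorded.
; IncrementDone raises the NumDone counter and, at the threshold, sets a one-shot MatThuSet flag before calling ShowMatthu.
; ShowMatthu finds every actor of the seven part classes and calls SetShow, then calls SetAsShow on all MatThu_Hint actors.
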(event `IncrementDone`
  (bind _result (`/Engine/EditorBlueprintResources/StandardMacros.IncrementInt` (`KismetMathLibrary.Conv_ByteToInt` (`self.NumDone`)))
    (:`  `
      (bind _output_get (set `self.NumDone` (`KismetMathLibrary.Conv_IntToByte` _result)))
      (if (and (>= (`self.NumDone`) 3) (not (`self.MatThuSet`)))
        (set `self.MatThuSet` true)
        (`self.ShowMatthu`)))))

(event `ShowMatthu`
  (`|ExecutionSequence`
    (:`then_0`
      (`|ExecutionSequence`
        (:`then_0`
          (bind _outactors (`GameplayStatics.GetAllActorsOfClass` "/Game/Blueprints/Mathu/FirstPart.FirstPart_C"))
          (for _array_element _outactors
            (`/Game/Blueprints/Mathu/FirstPart.setShow` _array_element)))
        (:`then_1`
          (bind _outactors_2 (`GameplayStatics.GetAllActorsOfClass` "/Game/Blueprints/Mathu/SecondPart.SecondPart_C"))
          (for _array_element_2 _outactors_2
            (`/Game/Blueprints/Mathu/SecondPart.setShow` _array_element_2)))
        (:`then_2`
          (bind _outactors_3 (`GameplayStatics.GetAllActorsOfClass` "/Game/Blueprints/Mathu/ThirdPart.ThirdPart_C"))
          (for _array_element_3 _outactors_3
            (`/Game/Blueprints/Mathu/ThirdPart.setShow` _array_element_3)))
        (:`then_3`
          (bind _outactors_4 (`GameplayStatics.GetAllActorsOfClass` "/Game/Blueprints/Mathu/FourthPart.FourthPart_C"))
          (for _array_element_4 _outactors_4
            (`/Game/Blueprints/Mathu/FourthPart.setShow` _array_element_4)))
        (:`then_4`
          (bind _outactors_5 (`GameplayStatics.GetAllActorsOfClass` "/Game/Blueprints/Mathu/FifthPart.FifthPart_C"))
          (for _array_element_5 _outactors_5
            (`/Game/Blueprints/Mathu/FifthPart.setShow` _array_element_5)))
        (:`then_5`
          (bind _outactors_6 (`GameplayStatics.GetAllActorsOfClass` "/Game/Blueprints/Mathu/SixthPart.SixthPart_C"))
          (for _array_element_6 _outactors_6
            (`/Game/Blueprints/Mathu/SixthPart.setShow` _array_element_6)))
        (:`then_6`
          (bind _outactors_7 (`GameplayStatics.GetAllActorsOfClass` "/Game/Blueprints/Mathu/SeventhPart.SeventhPart_C"))
          (for _array_element_7 _outactors_7
            (`/Game/Blueprints/Mathu/SeventhPart.setShow` _array_element_7)))))
    (:`then_1`
      (bind _outactors_8 (`GameplayStatics.GetAllActorsOfClass` "/Game/Blueprints/Mathu/MatThu_Hint.MatThu_Hint_C"))
      (for _array_element_8 _outactors_8
        (`/Game/Blueprints/Mathu/MatThu_Hint.SetAsShow` _array_element_8)))))

(fn `UserConstructionScript`)