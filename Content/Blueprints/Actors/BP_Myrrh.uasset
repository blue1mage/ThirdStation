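; BP_Myrrh is the myrrh actor, set up with that final name and a message asking for a gift that represents life or death.
; BeginPlay passes both strings to InitFunction, which is defined outside this graph.
; Tick polls IsDone and, the first time it is true, sets the CalledGM latch and calls IncrementDone on BP_GameMode.
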(event `self.ReceiveBeginPlay`
  (`self.initFunction` "myrrh" "Life or death. The Lord reign above all. I need a gift to represent that."))

(event `self.ReceiveTick`
  (params (DeltaSeconds :type "Float (single-precision)"))
  (bind _returnvalue (`self.IsDone`))
  (if (and _returnvalue (not (`self.CalledGM`)))
    (set `self.CalledGM` true)
    (bind _asbp_game_mode (cast `/Game/Blueprints/BP_GameMode` (`GameplayStatics.GetGameMode`)))
    (`/Game/Blueprints/BP_GameMode.IncrementDone` _asbp_game_mode)))

(fn `UserConstructionScript`)